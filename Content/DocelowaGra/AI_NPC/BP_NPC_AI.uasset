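; BP_NPC_AI is an NPC AI controller that records sighted resources.
; Sight perception updates sort actors tagged Drink or Shelter into arrays and increment counters, without checking duplicates or lost sight; the Shelter add has no actor wired.
; PruneFoodArray compacts null Food entries and updates the food count, though nothing here fills or prunes that array.
; The blackboard and behavior tree startup is disconnected, so it never runs.
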(event `self.AIPerception_Sight.OnTargetPerceptionUpdated`
  (params (Actor :type "Actor Object Reference") (Stimulus :type "AIStimulus Structure"))
  (if (`self.ActorHasTag` Actor "Drink")
    (`KismetArrayLibrary.Array_Add` (`self.Drink`) Actor)
    (set `self.HowMuchWater` (+ (`self.HowMuchWater`) 1))
    (elif (`self.ActorHasTag` Actor "Shelter")
      (`KismetArrayLibrary.Array_Add` (`self.Shelter`))
      (set `self.HowMuchShelter` (+ (`self.HowMuchShelter`) 1))
      (`KismetSystemLibrary.PrintString` (`KismetSystemLibrary.GetDisplayName` Actor)))))

(fn `PruneFoodArray`
  (bind _returnvalue (`MaslowBiologicalComponent.CompactNullActors` (`self.Food`)))
  (set `self.HowMuchFood` _returnvalue))

(fn `UserConstructionScript`)